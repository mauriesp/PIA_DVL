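; Ammo pickup actor that adds reserve ammo to the player's rifle when the player character overlaps its box.
; It raises MaxAmmo by a fixed amount on Rifle1 or Rifle2, depending on which is in use, and mirrors the value onto the character.
; It then matches itself against four ammo references on the character, sets the matching Taken flag, and destroys itself only if one matches.
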(event `self.ReceiveBeginPlay`)

(event `self.Box.OnComponentBeginOverlap`
  (params (OverlappedComponent :type "PrimitiveComponent Object Reference") (OtherActor :type "Actor Object Reference") (OtherComp :type "PrimitiveComponent Object Reference") (OtherBodyIndex :type Integer) (bFromSweep :type Boolean) (SweepResult :type "HitResult Structure (by ref)"))
  (bind _charref (`self.charRef`))
  (bind _asthird_person_character (cast `/Game/ThirdPersonBP/Blueprints/ThirdPersonCharacter` (`GameplayStatics.GetPlayerCharacter` 0)))
  (bind _output_get (set `self.charRef` _asthird_person_character))
  (if (== _output_get OtherActor)
    (if (`/Game/ThirdPersonBP/Blueprints/ThirdPersonCharacter.usingRifle1` _output_get)
      (bind _rifle1 (`/Game/ThirdPersonBP/Blueprints/ThirdPersonCharacter.Rifle1` _output_get))
      (bind _output_get_2 (set `/Game/Weapons/Rifle1/WeaponBase.MaxAmmo` (+ (`/Game/Weapons/Rifle1/WeaponBase.MaxAmmo` _rifle1) 5) _rifle1))
      (set `/Game/ThirdPersonBP/Blueprints/ThirdPersonCharacter.Rifle1MaxAmmo` _output_get_2 (`self.charRef`))
      (else
        (bind _rifle2 (`/Game/ThirdPersonBP/Blueprints/ThirdPersonCharacter.Rifle2` _output_get))
        (bind _output_get_3 (set `/Game/Weapons/Rifle2/WeaponBase2.MaxAmmo` (+ (`/Game/Weapons/Rifle2/WeaponBase2.MaxAmmo` _rifle2) 5) _rifle2))
        (set `/Game/ThirdPersonBP/Blueprints/ThirdPersonCharacter.Rifle2MaxAmmo` _output_get_3 (`self.charRef`))))
    (if (== self (`/Game/ThirdPersonBP/Blueprints/ThirdPersonCharacter.ammo1Ref` _charref))
      (set `/Game/ThirdPersonBP/Blueprints/ThirdPersonCharacter.ammo1Taken` true _charref)
      (`self.K2_DestroyActor`)
      (elif (== self (`/Game/ThirdPersonBP/Blueprints/ThirdPersonCharacter.ammo2Ref` _charref))
        (set `/Game/ThirdPersonBP/Blueprints/ThirdPersonCharacter.ammo2Taken` true _charref)
        (`self.K2_DestroyActor`)
        (elif (== self (`/Game/ThirdPersonBP/Blueprints/ThirdPersonCharacter.ammo3Ref` _charref))
          (set `/Game/ThirdPersonBP/Blueprints/ThirdPersonCharacter.ammo3Taken` true _charref)
          (`self.K2_DestroyActor`)
          (elif (== self (`/Game/ThirdPersonBP/Blueprints/ThirdPersonCharacter.ammo4Ref` _charref))
            (set `/Game/ThirdPersonBP/Blueprints/ThirdPersonCharacter.ammo4Taken` true _charref)
            (`self.K2_DestroyActor`)))))))

(fn `UserConstructionScript`)