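; Game instance that owns the player's save game in a single named slot.
; On Init it loads the existing slot or creates a new SaveGameObject in memory.
; SavePlayerData copies the third-person character's location, health, rifle ammo, pickup, cinematic and destroyed-object flags, and name into one struct and writes it to disk.
; LoadPlayerData applies that cached struct back to the character; ClearSavedData only deletes the slot.
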(event `self.ReceiveInit`
  (bind _returnvalue (`GameplayStatics.DoesSaveGameExist` (`self.SaveSlotName`)))
  (if _returnvalue
    (bind _returnvalue_2 (`GameplayStatics.LoadGameFromSlot` (`self.SaveSlotName`)))
    (bind _assave_game_object (cast `/Game/Blueprints/SaveGameObject` _returnvalue_2))
    (set `self.SaveGameData` _assave_game_object)
    (else
      (bind _returnvalue_3 (`GameplayStatics.CreateSaveGameObject` "/Game/Blueprints/SaveGameObject.SaveGameObject_C"))
      (set `self.SaveGameData` _returnvalue_3))))

(fn `ClearSavedData`
  (`GameplayStatics.DeleteGameInSlot` (`self.SaveSlotName`)))

(fn `LoadPlayerData`
  (locals (playerRef :type "/Game/ThirdPersonBP/Blueprints/ThirdPersonCharacter Object Reference"))
  (bind (_playersavedata_location _playersavedata_currenthealth _playersavedata_rifle1ammo _playersavedata_rifle1maxammo _playersavedata_rifle2ammo _playersavedata_rifle2maxammo _playersavedata_ammo1taken _playersavedata_ammo2taken _playersavedata_ammo3taken _playersavedata_ammo4taken _playersavedata_cinematic1played _playersavedata_cinematic2played _playersavedata_cinematic3played _playersavedata_object1destroyed _playersavedata_object2destroyed _playersavedata_object3destroyed _playersavedata_object4destroyed _playersavedata_object5destroyed _playersavedata_object6destroyed _playersavedata_object7destroyed _playersavedata_object8destroyed _playersavedata_object9destroyed _playersavedata_object10destroyed _playersavedata_object11destroyed _playersavedata_playername) (break `/Game/Blueprints/PlayerSaveData` (`/Game/Blueprints/SaveGameObject.PlayerSaveData` (`self.SaveGameData`))))
  (bind _asthird_person_character (cast `/Game/ThirdPersonBP/Blueprints/ThirdPersonCharacter` (`GameplayStatics.GetPlayerCharacter` 0)))
  (bind _output_get (set `local.playerRef` _asthird_person_character))
  (`Actor.K2_SetActorLocation` _output_get _playersavedata_location false false)
  (set `/Game/ThirdPersonBP/Blueprints/ThirdPersonCharacter.currentHealth` _playersavedata_currenthealth _output_get)
  (set `/Game/ThirdPersonBP/Blueprints/ThirdPersonCharacter.Rifle1Ammo` _playersavedata_rifle1ammo _output_get)
  (set `/Game/ThirdPersonBP/Blueprints/ThirdPersonCharacter.Rifle1MaxAmmo` _playersavedata_rifle1maxammo _output_get)
  (set `/Game/ThirdPersonBP/Blueprints/ThirdPersonCharacter.Rifle2Ammo` _playersavedata_rifle2ammo _output_get)
  (set `/Game/ThirdPersonBP/Blueprints/ThirdPersonCharacter.Rifle2MaxAmmo` _playersavedata_rifle2maxammo _output_get)
  (set `/Game/ThirdPersonBP/Blueprints/ThirdPersonCharacter.ammo1Taken` _playersavedata_ammo1taken _output_get)
  (set `/Game/ThirdPersonBP/Blueprints/ThirdPersonCharacter.ammo2Taken` _playersavedata_ammo2taken _output_get)
  (set `/Game/ThirdPersonBP/Blueprints/ThirdPersonCharacter.ammo3Taken` _playersavedata_ammo3taken _output_get)
  (set `/Game/ThirdPersonBP/Blueprints/ThirdPersonCharacter.ammo4Taken` _playersavedata_ammo4taken _output_get)
  (set `/Game/ThirdPersonBP/Blueprints/ThirdPersonCharacter.cinematic1Played` _playersavedata_cinematic1played _output_get)
  (set `/Game/ThirdPersonBP/Blueprints/ThirdPersonCharacter.cinematic2Played` _playersavedata_cinematic2played _output_get)
  (set `/Game/ThirdPersonBP/Blueprints/ThirdPersonCharacter.cinematic3Played` _playersavedata_cinematic3played _output_get)
  (set `/Game/ThirdPersonBP/Blueprints/ThirdPersonCharacter.object1Destroyed` _playersavedata_object1destroyed _output_get)
  (set `/Game/ThirdPersonBP/Blueprints/ThirdPersonCharacter.object2Destroyed` _playersavedata_object2destroyed _output_get)
  (set `/Game/ThirdPersonBP/Blueprints/ThirdPersonCharacter.object3Destroyed` _playersavedata_object3destroyed _output_get)
  (set `/Game/ThirdPersonBP/Blueprints/ThirdPersonCharacter.object4Destroyed` _playersavedata_object4destroyed _output_get)
  (set `/Game/ThirdPersonBP/Blueprints/ThirdPersonCharacter.object5Destroyed` _playersavedata_object5destroyed _output_get)
  (set `/Game/ThirdPersonBP/Blueprints/ThirdPersonCharacter.object6Destroyed` _playersavedata_object6destroyed _output_get)
  (set `/Game/ThirdPersonBP/Blueprints/ThirdPersonCharacter.object7Destroyed` _playersavedata_object7destroyed _output_get)
  (set `/Game/ThirdPersonBP/Blueprints/ThirdPersonCharacter.object8Destroyed` _playersavedata_object8destroyed _output_get)
  (set `/Game/ThirdPersonBP/Blueprints/ThirdPersonCharacter.object9Destroyed` _playersavedata_object9destroyed _output_get)
  (set `/Game/ThirdPersonBP/Blueprints/ThirdPersonCharacter.object10Destroyed` _playersavedata_object10destroyed _output_get)
  (set `/Game/ThirdPersonBP/Blueprints/ThirdPersonCharacter.object11Destroyed` _playersavedata_object11destroyed _output_get)
  (set `/Game/ThirdPersonBP/Blueprints/ThirdPersonCharacter.playerName` _playersavedata_playername _output_get))

(fn `SavePlayerData`
  (locals (playerRef :type "/Game/ThirdPersonBP/Blueprints/ThirdPersonCharacter Object Reference"))
  (bind _asthird_person_character (cast `/Game/ThirdPersonBP/Blueprints/ThirdPersonCharacter` (`GameplayStatics.GetPlayerCharacter` 0)))
  (bind _output_get (set `local.playerRef` _asthird_person_character))
  (set `/Game/Blueprints/SaveGameObject.PlayerSaveData` (make `/Game/Blueprints/PlayerSaveData` (`Actor.K2_GetActorLocation` _output_get) (`/Game/ThirdPersonBP/Blueprints/ThirdPersonCharacter.currentHealth` _output_get) (`/Game/ThirdPersonBP/Blueprints/ThirdPersonCharacter.Rifle1Ammo` _output_get) (`/Game/ThirdPersonBP/Blueprints/ThirdPersonCharacter.Rifle1MaxAmmo` _output_get) (`/Game/ThirdPersonBP/Blueprints/ThirdPersonCharacter.Rifle2Ammo` _output_get) (`/Game/ThirdPersonBP/Blueprints/ThirdPersonCharacter.Rifle2MaxAmmo` _output_get) (`/Game/ThirdPersonBP/Blueprints/ThirdPersonCharacter.ammo1Taken` _output_get) (`/Game/ThirdPersonBP/Blueprints/ThirdPersonCharacter.ammo2Taken` _output_get) (`/Game/ThirdPersonBP/Blueprints/ThirdPersonCharacter.ammo3Taken` _output_get) (`/Game/ThirdPersonBP/Blueprints/ThirdPersonCharacter.ammo4Taken` _output_get) (`/Game/ThirdPersonBP/Blueprints/ThirdPersonCharacter.cinematic1Played` _output_get) (`/Game/ThirdPersonBP/Blueprints/ThirdPersonCharacter.cinematic2Played` _output_get) (`/Game/ThirdPersonBP/Blueprints/ThirdPersonCharacter.cinematic3Played` _output_get) (`/Game/ThirdPersonBP/Blueprints/ThirdPersonCharacter.object1Destroyed` _output_get) (`/Game/ThirdPersonBP/Blueprints/ThirdPersonCharacter.object2Destroyed` _output_get) (`/Game/ThirdPersonBP/Blueprints/ThirdPersonCharacter.object3Destroyed` _output_get) (`/Game/ThirdPersonBP/Blueprints/ThirdPersonCharacter.object4Destroyed` _output_get) (`/Game/ThirdPersonBP/Blueprints/ThirdPersonCharacter.object5Destroyed` _output_get) (`/Game/ThirdPersonBP/Blueprints/ThirdPersonCharacter.object6Destroyed` _output_get) (`/Game/ThirdPersonBP/Blueprints/ThirdPersonCharacter.object7Destroyed` _output_get) (`/Game/ThirdPersonBP/Blueprints/ThirdPersonCharacter.object8Destroyed` _output_get) (`/Game/ThirdPersonBP/Blueprints/ThirdPersonCharacter.object9Destroyed` _output_get) (`/Game/ThirdPersonBP/Blueprints/ThirdPersonCharacter.object10Destroyed` _output_get) (`/Game/ThirdPersonBP/Blueprints/ThirdPersonCharacter.object11Destroyed` _output_get) (`/Game/ThirdPersonBP/Blueprints/ThirdPersonCharacter.playerName` _output_get)) (`self.SaveGameData`))
  (`GameplayStatics.SaveGameToSlot` (`self.SaveGameData`) (`self.SaveSlotName`)))